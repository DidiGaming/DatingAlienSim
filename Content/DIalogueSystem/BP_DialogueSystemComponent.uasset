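; BP_DialogueSystemComponent is a skeleton dialogue component with functions for reading the current question and its answers and for proceeding on an answer.
; GetCurrentQuestion, GetCurrentAnswers and ProceedAnswer return only empty or default values, and IsCurrentGroupID has no logic.
; On BeginPlay, debug code prints the current question, then each key and value from the answers map in a contrasting colour.
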(event `self.ReceiveBeginPlay`
  ;[1 1 1] Debug Info
  (bind _question (`self.GetCurrentQuestion`))
  (`KismetSystemLibrary.PrintString` (`KismetTextLibrary.Conv_TextToString` _question) true true (struct :`G` 0.66 :`B` 1.0 :`A` 1.0) 10.0)
  (bind _answers (`self.GetCurrentAnswers`))
  (bind _keys (`BlueprintMapLibrary.Map_Keys` _answers))
  (for _array_element _keys
    (bind (_value _returnvalue) (`BlueprintMapLibrary.Map_Find` _answers _array_element))
    (if _returnvalue
      (`KismetSystemLibrary.PrintString` (`KismetStringLibrary.Concat_StrStr` (`KismetStringLibrary.Conv_IntToString` _array_element) (`KismetTextLibrary.Conv_TextToString` _value)) true true (struct :`R` 1.0 :`G` 0.018288 :`B` 0.332501 :`A` 1.0) 10.0))))

(fn `GetCurrentAnswers`
  (returns (Answers :type "Map of Integer to Text"))
  (return))

(fn `GetCurrentQuestion`
  (returns (Question :type Text))
  (return ""))

(fn `ProceedAnswer`
  (returns (AnsweID :type Integer))
  (return 0))