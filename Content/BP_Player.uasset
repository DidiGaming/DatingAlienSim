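; Player Blueprint for a Jabba the Hutt scene, showing the cursor with UI-only input and controlling the backdrop and Jabba's mood.
; SwitchScreen swaps the material and plays a sound on the first StaticMeshActor found, cached as the background.
; SetJabbaMood maps each mood to a sprite and sound.
; BeginPlay runs a timed, hard-coded sequence that changes the backdrop to Tatooine and cycles through every mood.
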(event `self.ReceiveBeginPlay`
  (bind _returnvalue (`GameplayStatics.GetPlayerController` 0))
  (`|ExecutionSequence`
    (:`then_0`
      (set `PlayerController.bShowMouseCursor` true _returnvalue)
      (`WidgetBlueprintLibrary.SetInputMode_UIOnlyEx` _returnvalue null))
    (:`then_1`
      (`KismetSystemLibrary.Delay` 5.0)
      (`self.SwitchScreen` "/Game/Enviroment/M_Tatooine_02.M_Tatooine_02"))
    (:`then_2`
      (bind _returnvalue_2 (`GameplayStatics.GetActorOfClass` "/Script/Engine.StaticMeshActor"))
      (set `self.Background` _returnvalue_2))
    (:`then_3`
      (`self.SetJabbaMood` "NewEnumerator0")
      (`KismetSystemLibrary.Delay` 4.0)
      (`self.SetJabbaMood` "NewEnumerator1")
      (`KismetSystemLibrary.Delay` 4.0)
      (`self.SetJabbaMood` "NewEnumerator2")
      (`KismetSystemLibrary.Delay` 4.0)
      (`self.SetJabbaMood` "NewEnumerator3")
      (`KismetSystemLibrary.Delay` 4.0)
      (`self.SetJabbaMood` "NewEnumerator4"))))

(event `SwitchScreen`
  (params (`Scene Material` :type "MaterialInterface Object Reference") (`Scene Sound` :type "SoundBase Object Reference"))
  ;[1 1 1] Switch Scene
  (`/Engine/EditorBlueprintResources/StandardMacros.IsValid` (`self.Background`)
    (:`Is Valid`
      (`PrimitiveComponent.SetMaterial` (`StaticMeshActor.StaticMeshComponent` (`self.Background`)) 0 `Scene Material`)
      (`GameplayStatics.PlaySound2D` `Scene Sound` 1.0 1.0 0.0 null null))))

(fn `SetJabbaMood`
  (params (`New Mood` :type "/Game/ST_Jabba_MoodStates Enum" :default "NewEnumerator0"))
  (switch `/Game/ST_Jabba_MoodStates` `New Mood`
    (:`NewEnumerator0`
      (`PaperSpriteComponent.SetSprite` (`self.Jabba`) (`self.Jabba_Normal`))
      (`GameplayStatics.PlaySound2D` "/Game/Sound/Jabba_Sad.Jabba_Sad" 2.0 1.0 0.0 null null))
    (:`NewEnumerator1`
      (`PaperSpriteComponent.SetSprite` (`self.Jabba`) (`self.Jabba_Happy`))
      (`GameplayStatics.PlaySound2D` "/Game/Sound/Jabba-The-Hutt-Laughing_Star-wars_-Sound-Effect.Jabba-The-Hutt-Laughing_Star-wars_-Sound-Effect" 0.5 1.0 0.0 null null))
    (:`NewEnumerator2`
      (`PaperSpriteComponent.SetSprite` (`self.Jabba`) (`self.Jabba_Angry`))
      (`GameplayStatics.PlaySound2D` "/Game/Sound/Jabba_Angry.Jabba_Angry" 1.5 1.0 0.0 null null))
    (:`NewEnumerator3`
      (`PaperSpriteComponent.SetSprite` (`self.Jabba`) (`self.Jabba_Sad`))
      (`GameplayStatics.PlaySound2D` "/Game/Sound/Jabba_Sad.Jabba_Sad" 1.5 1.0 0.0 null null))
    (:`NewEnumerator4`
      (`PaperSpriteComponent.SetSprite` (`self.Jabba`) (`self.Jabba_Horny`))
      (`GameplayStatics.PlaySound2D` "/Game/Sound/Jabba_Horny.Jabba_Horny" 1.2 1.0 0.0 null null))))

(fn `UserConstructionScript`)